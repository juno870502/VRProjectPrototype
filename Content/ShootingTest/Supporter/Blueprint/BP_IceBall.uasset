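; BP_IceBall is an ice ball projectile that is summoned at a socket and then shot in a given direction.
; SummonTheBall handles socket attachment using the passed Parent component and socket name, keeping relative transforms.
; ShootTheBall switches the Sphere to the Projectile collision profile and hands it to ProjectileMovement with velocity, bouncing and a short lifespan.
; The file has no hit or damage logic.
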(event `self.ReceiveBeginPlay`)

(event `ShootTheBall`
  (params (ShootDirection :type "Vector Structure"))
  (bind _sphere (`self.Sphere`))
  (bind _projectilemovement (`self.ProjectileMovement`))
  (`PrimitiveComponent.SetCollisionProfileName` _sphere "Projectile")
  (set `MovementComponent.Velocity` (* ShootDirection (`ProjectileMovementComponent.InitialSpeed` _projectilemovement)) _projectilemovement)
  (`MovementComponent.SetUpdatedComponent` _projectilemovement _sphere)
  (set `ProjectileMovementComponent.bRotationFollowsVelocity` true _projectilemovement)
  (set `ProjectileMovementComponent.bShouldBounce` true _projectilemovement)
  (`self.SetLifeSpan` 5.0))

(event `SummonTheBall`
  (params (Parent :type "SceneComponent Object Reference") (SocketName :type Name))
  (`SceneComponent.K2_AttachToComponent` Parent null SocketName "KeepRelative" "KeepRelative" "KeepRelative" false))

(fn `UserConstructionScript`)