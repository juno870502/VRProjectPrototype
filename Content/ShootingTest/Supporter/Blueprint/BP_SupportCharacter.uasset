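; BP_SupportCharacter is a support character that casts ice magic, with yaw and pitch look input and two select actions to switch spells.
; Pressing Fire branches on the selected spell: Ice Bolt spawns at Arrow1 and shoots immediately, while Ice Ball spawns attached to the mesh's GripPoint socket.
; Releasing Fire detaches a held Ice Ball and launches it along the actor's forward vector, giving that spell a hold-and-release cast.
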(event `self.ReceiveTick`
  (params (DeltaSeconds :type "Float (single-precision)")))

(event `InputAxis|Turn`
  (params (AxisValue :type "Float (single-precision)"))
  (`self.AddControllerYawInput` AxisValue))

(event `InputAxis|LookUp`
  (params (AxisValue :type "Float (single-precision)"))
  (`self.AddControllerPitchInput` AxisValue))

(event `InputAction|Fire`
  (params (Key :type "Key Structure"))
  (:`Pressed`
    (`self.FirePressed`))
  (:`Released`
    (`self.FireReleased`)))

(event `InputAction|Select First Magic`
  (params (Key :type "Key Structure"))
  ;[0 0.271 1] Select Magic Event
  (:`Pressed`
    (set `self.Kind of IceMagic` "NewEnumerator0")))

(event `InputAction|Select Second Magic`
  (params (Key :type "Key Structure"))
  ;[0 0.271 1] Select Magic Event
  (:`Pressed`
    (set `self.Kind of IceMagic` "NewEnumerator1")))

(fn `FirePressed`
  (switch `/Game/ShootingTest/Supporter/Blueprint/Enum_IceMagic` (`self.Kind of IceMagic`)
    (:`NewEnumerator0`
      (bind _returnvalue (`|SpawnActorFromClass` "/Game/ShootingTest/Supporter/Blueprint/BP_IceBolt.BP_IceBolt_C" (`SceneComponent.K2_GetComponentToWorld` (`self.Arrow1`)) "Undefined" "OverrideRootScale" null null))
      (`/Game/ShootingTest/Supporter/Blueprint/BP_IceBolt.ShootMagic` _returnvalue (`SceneComponent.GetForwardVector` (`self.Arrow1`))))
    (:`NewEnumerator1`
      (bind _returnvalue_2 (`|SpawnActorFromClass` "/Game/ShootingTest/Supporter/Blueprint/BP_IceBall.BP_IceBall_C" (`SceneComponent.GetSocketTransform` (`self.Mesh`) "GripPoint" "RTS_ParentBoneSpace") "Undefined" "OverrideRootScale" null null))
      (set `self.SpawnActor` _returnvalue_2)
      (`self.K2_AttachToComponent` (`self.SpawnActor`) (`self.Mesh`) "GripPoint" "KeepRelative" "KeepRelative" "KeepRelative" true))))

(fn `FireReleased`
  (bind _spawnactor (`self.SpawnActor`))
  (switch `/Game/ShootingTest/Supporter/Blueprint/Enum_IceMagic` (`self.Kind of IceMagic`)
    (:`NewEnumerator1`
      (if (`KismetSystemLibrary.IsValid` _spawnactor)
        (`self.K2_DetachFromActor` _spawnactor "KeepWorld" "KeepWorld" "KeepWorld")
        (message `/Game/ShootingTest/Supporter/Blueprint/BPI_IceMagic.ShootMagic` _spawnactor (`self.GetActorForwardVector`))))))

(fn `UserConstructionScript`)