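; BP_IceBolt is an ice bolt magic projectile in the ShootingTest Supporter folder that homes in on tagged targets.
; ShootMagic launches it along a given direction through ProjectileMovement on the Sphere, with bouncing, velocity-aligned rotation and a limited lifespan.
; A SensingCollision overlap with an actor tagged "Target" turns on homing toward the overlapped component, so the bolt flies straight until it detects one.
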(event `/Game/ShootingTest/Supporter/Blueprint/BPI_IceMagic.ShootMagic`
  (params (Direction :type "Vector Structure"))
  (bind _projectilemovement (`self.ProjectileMovement`))
  (set `MovementComponent.Velocity` (* Direction 500.0) _projectilemovement)
  (`MovementComponent.SetUpdatedComponent` _projectilemovement (`self.Sphere`))
  (set `ProjectileMovementComponent.bRotationFollowsVelocity` true _projectilemovement)
  (set `ProjectileMovementComponent.bShouldBounce` true _projectilemovement)
  (`self.SetLifeSpan` 5.0))

(event `self.SensingCollision.OnComponentBeginOverlap`
  (params (OverlappedComponent :type "PrimitiveComponent Object Reference") (OtherActor :type "Actor Object Reference") (OtherComp :type "PrimitiveComponent Object Reference") (OtherBodyIndex :type Integer) (bFromSweep :type Boolean) (SweepResult :type "HitResult Structure (by ref)"))
  (bind _projectilemovement (`self.ProjectileMovement`))
  (if (`self.ActorHasTag` OtherActor "Target")
    (set `ProjectileMovementComponent.HomingTargetComponent` OtherComp _projectilemovement)
    (set `ProjectileMovementComponent.bIsHomingProjectile` true _projectilemovement)
    (set `ProjectileMovementComponent.HomingAccelerationMagnitude` 1500.0 _projectilemovement)))

(fn `UserConstructionScript`)